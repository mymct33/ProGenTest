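; BP_LevelGenerator builds a random grid-based level of connected rooms, replacing any rooms it spawned before.
; SetVariables random-walks from the grid centre, backtracking at dead ends or by chance to form branches, and records each room's connections.
; It mirrors those links, attempts extra connections between neighbours to create loops, then spawns rotated room Blueprints matching each cell's entry count and shape.
; Finally, it issues a RebuildNavigation console command.
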(event Custom|SetVariables
  (params (StartingPos :type Vector) (LevelDimensions :type Vector%202D%20Structure) (RoomDimensions :type Vector%202D%20Structure) (NumberOfRooms :type Integer) (BranchChance :type Float%20%28single-precision%29) (ExtraConnections :type Integer) (MaxBranchLength :type Integer))
  (bind _returnvalue (Math|Random|RandomInteger 2))
  (bind _rooms (Variables|Default|GetRooms))
  (bind _rooms_2 (Variables|Default|GetRooms))
  (bind _movedirections (Variables|Movement|GetMoveDirections))
  (bind _movedirections_2 (Variables|Movement|GetMoveDirections))
  (bind _movedirections_3 (Variables|Movement|GetMoveDirections))
  (bind _movedirections_4 (Variables|Movement|GetMoveDirections))
  (bind _roomplaced (Variables|Default|GetRoomPlaced))
  (bind _connectedrooms (Variables|Default|GetConnectedRooms))
  (bind _roomplaced_2 (Variables|Default|GetRoomPlaced))
  (bind _movedirections_5 (Variables|Movement|GetMoveDirections))
  ;[1 1 1] Set Variables
  (Variables|LevelProperties|SetStartingPos StartingPos)
  (Variables|LevelProperties|SetLevelDimensions LevelDimensions)
  (Variables|LevelProperties|SetRoomDimensions RoomDimensions)
  (Variables|LevelProperties|SetNumberOfRooms NumberOfRooms)
  (Variables|LevelProperties|SetBranchChance BranchChance)
  (Variables|LevelProperties|SetExtraConnections ExtraConnections)
  (Variables|LevelProperties|SetMaxBranchLength MaxBranchLength)
  (Variables|Default|SetPreviousRoom -1)
  (Utilities|Array|Clear (Variables|Movement|GetStepsTaken))
  (Variables|LevelProperties|SetLevelDimensionsX (Math|Float|Floor (.X (Math|Vector2D|BreakVector2D (Variables|LevelProperties|GetLevelDimensions)))))
  (Variables|LevelProperties|SetLevelDimensionsY (Math|Float|Floor (.Y (Math|Vector2D|BreakVector2D (Variables|LevelProperties|GetLevelDimensions)))))
  (for _array_element _rooms_2
    (Actor|DestroyActor _array_element))
  (Utilities|Array|Clear _rooms_2)
  (Utilities|Array|Resize _rooms_2 (* (Variables|LevelProperties|GetLevelDimensionsX) (Variables|LevelProperties|GetLevelDimensionsY)))
  (Utilities|Array|Clear _roomplaced)
  (Utilities|Array|Resize _roomplaced (* (Variables|LevelProperties|GetLevelDimensionsX) (Variables|LevelProperties|GetLevelDimensionsY)))
  (Utilities|Array|Clear _connectedrooms)
  (Utilities|Array|Resize _connectedrooms (* (Variables|LevelProperties|GetLevelDimensionsX) (Variables|LevelProperties|GetLevelDimensionsY)))
  (bind _arrayposition (CallFunction|2DCoordsto1DArray (Math|Float|Floor (* (.X (Math|Vector2D|BreakVector2D (Variables|LevelProperties|GetLevelDimensions))) 0.5)) (Math|Float|Floor (* (.Y (Math|Vector2D|BreakVector2D (Variables|LevelProperties|GetLevelDimensions))) 0.5)) (Variables|LevelProperties|GetLevelDimensionsX)))
  (Variables|Default|SetCurrentRoom _arrayposition)
  (bind _index (Utilities|FlowControl|ForLoopwithBreak 1 (Variables|LevelProperties|GetNumberOfRooms) :!label _label)
    (:LoopBody
      (Variables|Default|SetMainLoopIndex _index)
      ;[1 1 1] Allocate Room
      (Utilities|Array|Add (Variables|Movement|GetStepsTaken) (Variables|Default|GetCurrentRoom))
      (Utilities|Array|SetArrayElem (Variables|Default|GetRoomPlaced) (Variables|Default|GetCurrentRoom) true)
      ;[1 1 1] If First Room
      (if (== (Variables|Default|GetPreviousRoom) -1)
        _
        (else
          ;[1 1 1] Inform About Connected Room (Stage 1)
          (Utilities|Array|SetArrayElem (Variables|Default|GetConnectedRooms) (Variables|Default|GetCurrentRoom) (Utilities|Struct|MakeSTRUCT_ConnectedRooms (== (- (Variables|Default|GetCurrentRoom) (Variables|Default|GetPreviousRoom)) 1) (== (- (Variables|Default|GetCurrentRoom) (Variables|Default|GetPreviousRoom)) -1) (== (- (Variables|Default|GetCurrentRoom) (Variables|Default|GetPreviousRoom)) (Variables|LevelProperties|GetLevelDimensionsX)) (== (- (Variables|Default|GetCurrentRoom) (Variables|Default|GetPreviousRoom)) (* (Variables|LevelProperties|GetLevelDimensionsX) -1))))
          ;[1 1 1] Check if map is full
          (if (< (Utilities|Array|Length (Variables|Movement|GetStepsTaken)) (* (Variables|LevelProperties|GetLevelDimensionsX) (Variables|LevelProperties|GetLevelDimensionsY)))
            ;[1 1 1] Random chance to step back
            (if (> (Math|Random|RandomFloat) (Variables|LevelProperties|GetBranchChance))
              _
              (else
                (Variables|Default|SetMainLoopIndex (Math|Integer|Max(Integer) (- (Variables|Default|GetMainLoopIndex) (Math|Random|RandomIntegerinRange 1 (Variables|LevelProperties|GetMaxBranchLength)))))
                (Variables|Default|SetCurrentRoom (Utilities|Array|Get(acopy) (Variables|Movement|GetStepsTaken) (Variables|Default|GetMainLoopIndex)))))
            (else
              (goto _label Break)))))
      ;[1 1 1] Check Where We Can Move Next
      (Utilities|FlowControl|Sequence :!label _label_2
        (:then_0
          ;;[1 1 1] Left
          (if (> (Math|Integer|%(Integer) (Variables|Default|GetCurrentRoom) (Variables|LevelProperties|GetLevelDimensionsX)) 0)
            (if (Utilities|Array|Get(acopy) (Variables|Default|GetRoomPlaced) (- (Variables|Default|GetCurrentRoom) 1))
              (Utilities|Array|Add _movedirections_2 false :!label _label_3)
              (else
                (Utilities|Array|Add _movedirections_2 true)))
            (else
              (goto _label_3))))
        (:then_1
          ;;[1 1 1] Right
          (if (< (Math|Integer|%(Integer) (Variables|Default|GetCurrentRoom) (Variables|LevelProperties|GetLevelDimensionsX)) (- (Variables|LevelProperties|GetLevelDimensionsX) 1))
            (if (Utilities|Array|Get(acopy) (Variables|Default|GetRoomPlaced) (+ (Variables|Default|GetCurrentRoom) 1))
              (Utilities|Array|Add _movedirections_3 false :!label _label_4)
              (else
                (Utilities|Array|Add _movedirections_3 true)))
            (else
              (goto _label_4))))
        (:then_2
          ;;[1 1 1] Up
          (if (>= (Variables|Default|GetCurrentRoom) (Variables|LevelProperties|GetLevelDimensionsX))
            (if (Utilities|Array|Get(acopy) (Variables|Default|GetRoomPlaced) (- (Variables|Default|GetCurrentRoom) (Variables|LevelProperties|GetLevelDimensionsX)))
              (Utilities|Array|Add _movedirections_4 false :!label _label_5)
              (else
                (Utilities|Array|Add _movedirections_4 true)))
            (else
              (goto _label_5))))
        (:then_3
          ;;[1 1 1] Down
          (if (< (Variables|Default|GetCurrentRoom) (* (Variables|LevelProperties|GetLevelDimensionsX) (- (Variables|LevelProperties|GetLevelDimensionsY) 1)))
            (if (Utilities|Array|Get(acopy) (Variables|Default|GetRoomPlaced) (+ (Variables|Default|GetCurrentRoom) (Variables|LevelProperties|GetLevelDimensionsX)))
              (Utilities|Array|Add _movedirections false :!label _label_6)
              (else
                (Utilities|Array|Add _movedirections true)))
            (else
              (goto _label_6))))
        (:then_4
          ;[1 1 1] Count Number of Move Options
          (Utilities|CheckMoveOptions
            (:Choose
              ;[1 1 1] Choose Random Direction to Move
              (Variables|Movement|SetMovementChoice (Math|Random|RandomIntegerinRange 1 (Variables|Movement|GetNoOfMoveOptions)))
              (for (_array_element_2 _array_index) (Variables|Movement|GetMoveDirections)
                (if _array_element_2
                  (Variables|Movement|SetMovementDirectionSearch (+ (Variables|Movement|GetMovementDirectionSearch) 1))
                  (if (== (Variables|Movement|GetMovementDirectionSearch) (Variables|Movement|GetMovementChoice))
                    (Variables|Default|SetPreviousRoom (Variables|Default|GetCurrentRoom))
                    (Variables|Default|SetCurrentRoom (Utilities|Select :Index _array_index :Option%200 (- (Variables|Default|GetCurrentRoom) 1) :Option%201 (+ (Variables|Default|GetCurrentRoom) 1) :Option%202 (- (Variables|Default|GetCurrentRoom) (Variables|LevelProperties|GetLevelDimensionsX)) :Option%203 (+ (Variables|Default|GetCurrentRoom) (Variables|LevelProperties|GetLevelDimensionsX))))
                    ;[1 1 1] Reset Variables
                    (Utilities|Array|Clear (Variables|Movement|GetMoveDirections))
                    (Variables|Movement|SetNoOfMoveOptions 0)
                    (Variables|Movement|SetMovementDirectionSearch 0)))))
            (:Try%20Again
              (Variables|Default|SetMainLoopIndex (- (Variables|Default|GetMainLoopIndex) 1))
              (Variables|Default|SetCurrentRoom (Utilities|Array|Get(acopy) (Variables|Movement|GetStepsTaken) (Variables|Default|GetMainLoopIndex)))
              ;[1 1 1] Reset before break
              (Utilities|Array|Clear (Variables|Movement|GetMoveDirections))
              (Variables|Movement|SetNoOfMoveOptions 0)
              (goto _label_2))))))
    (:Completed
      (Utilities|FlowControl|Sequence
        (:then_0
          ;[1 1 1] Inform About Connected Room (Stage 2)
          (for _array_element_3 (Variables|Movement|GetStepsTaken)
            (Variables|Default|SetMainLoopIndex _array_element_3)
            (Utilities|FlowControl|Sequence
              (:then_0
                (if (.Left (Utilities|Struct|BreakSTRUCT_ConnectedRooms (Utilities|Array|Get(acopy) (Variables|Default|GetConnectedRooms) (Variables|Default|GetMainLoopIndex))))
                  (Utilities|Array|SetArrayElem (Variables|Default|GetConnectedRooms) (- (Variables|Default|GetMainLoopIndex) 1) (Utilities|Struct|MakeSTRUCT_ConnectedRooms (.Left (Utilities|Struct|BreakSTRUCT_ConnectedRooms (Utilities|Array|Get(acopy) (Variables|Default|GetConnectedRooms) (- (Variables|Default|GetMainLoopIndex) 1)))) true (.Up (Utilities|Struct|BreakSTRUCT_ConnectedRooms (Utilities|Array|Get(acopy) (Variables|Default|GetConnectedRooms) (- (Variables|Default|GetMainLoopIndex) 1)))) (.Down (Utilities|Struct|BreakSTRUCT_ConnectedRooms (Utilities|Array|Get(acopy) (Variables|Default|GetConnectedRooms) (- (Variables|Default|GetMainLoopIndex) 1))))))))
              (:then_1
                (if (.Right (Utilities|Struct|BreakSTRUCT_ConnectedRooms (Utilities|Array|Get(acopy) (Variables|Default|GetConnectedRooms) (Variables|Default|GetMainLoopIndex))))
                  (Utilities|Array|SetArrayElem (Variables|Default|GetConnectedRooms) (+ (Variables|Default|GetMainLoopIndex) 1) (Utilities|Struct|MakeSTRUCT_ConnectedRooms true (.Right (Utilities|Struct|BreakSTRUCT_ConnectedRooms (Utilities|Array|Get(acopy) (Variables|Default|GetConnectedRooms) (+ (Variables|Default|GetMainLoopIndex) 1)))) (.Up (Utilities|Struct|BreakSTRUCT_ConnectedRooms (Utilities|Array|Get(acopy) (Variables|Default|GetConnectedRooms) (+ (Variables|Default|GetMainLoopIndex) 1)))) (.Down (Utilities|Struct|BreakSTRUCT_ConnectedRooms (Utilities|Array|Get(acopy) (Variables|Default|GetConnectedRooms) (+ (Variables|Default|GetMainLoopIndex) 1))))))))
              (:then_2
                (if (.Up (Utilities|Struct|BreakSTRUCT_ConnectedRooms (Utilities|Array|Get(acopy) (Variables|Default|GetConnectedRooms) (Variables|Default|GetMainLoopIndex))))
                  (Utilities|Array|SetArrayElem (Variables|Default|GetConnectedRooms) (- (Variables|Default|GetMainLoopIndex) (Variables|LevelProperties|GetLevelDimensionsX)) (Utilities|Struct|MakeSTRUCT_ConnectedRooms (.Left (Utilities|Struct|BreakSTRUCT_ConnectedRooms (Utilities|Array|Get(acopy) (Variables|Default|GetConnectedRooms) (- (Variables|Default|GetMainLoopIndex) (Variables|LevelProperties|GetLevelDimensionsX))))) (.Right (Utilities|Struct|BreakSTRUCT_ConnectedRooms (Utilities|Array|Get(acopy) (Variables|Default|GetConnectedRooms) (- (Variables|Default|GetMainLoopIndex) (Variables|LevelProperties|GetLevelDimensionsX))))) (.Up (Utilities|Struct|BreakSTRUCT_ConnectedRooms (Utilities|Array|Get(acopy) (Variables|Default|GetConnectedRooms) (- (Variables|Default|GetMainLoopIndex) (Variables|LevelProperties|GetLevelDimensionsX))))) true))))
              (:then_3
                (if (.Down (Utilities|Struct|BreakSTRUCT_ConnectedRooms (Utilities|Array|Get(acopy) (Variables|Default|GetConnectedRooms) (Variables|Default|GetMainLoopIndex))))
                  (Utilities|Array|SetArrayElem (Variables|Default|GetConnectedRooms) (+ (Variables|Default|GetMainLoopIndex) (Variables|LevelProperties|GetLevelDimensionsX)) (Utilities|Struct|MakeSTRUCT_ConnectedRooms (.Left (Utilities|Struct|BreakSTRUCT_ConnectedRooms (Utilities|Array|Get(acopy) (Variables|Default|GetConnectedRooms) (+ (Variables|Default|GetMainLoopIndex) (Variables|LevelProperties|GetLevelDimensionsX))))) (.Right (Utilities|Struct|BreakSTRUCT_ConnectedRooms (Utilities|Array|Get(acopy) (Variables|Default|GetConnectedRooms) (+ (Variables|Default|GetMainLoopIndex) (Variables|LevelProperties|GetLevelDimensionsX))))) true (.Down (Utilities|Struct|BreakSTRUCT_ConnectedRooms (Utilities|Array|Get(acopy) (Variables|Default|GetConnectedRooms) (+ (Variables|Default|GetMainLoopIndex) (Variables|LevelProperties|GetLevelDimensionsX))))))))))))
        (:then_1
          ;[1 1 1] Randomly Connect Rooms Together
          (Utilities|FlowControl|ForLoopwithBreak 1 (Variables|LevelProperties|GetExtraConnections) :!label _label_7
            (:LoopBody
              (Variables|Default|SetExtraConnectionAttempts 0)
              (Variables|Default|SetCurrentRoom (Utilities|Array|Get(acopy) (Variables|Movement|GetStepsTaken) (Math|Random|RandomInteger (Variables|LevelProperties|GetNumberOfRooms))) :!label _label_8)
              (Variables|Default|SetExtraConnectionAttempts (+ (Variables|Default|GetExtraConnectionAttempts) 1))
              (Utilities|FlowControl|Sequence
                (:then_0
                  (if (> (Math|Integer|%(Integer) (Variables|Default|GetCurrentRoom) (Variables|LevelProperties|GetLevelDimensionsX)) 0)
                    (if (.Left (Utilities|Struct|BreakSTRUCT_ConnectedRooms (Utilities|Array|Get(acopy) (Variables|Default|GetConnectedRooms) (Variables|Default|GetCurrentRoom))))
                      (Utilities|Array|Add (Variables|Movement|GetMoveDirections) false :!label _label_9)
                      (else
                        (Utilities|Array|Add _movedirections_5 (Utilities|Array|Get(acopy) _roomplaced_2 (- (Variables|Default|GetCurrentRoom) 1)))))
                    (else
                      (goto _label_9))))
                (:then_1
                  (if (< (Math|Integer|%(Integer) (Variables|Default|GetCurrentRoom) (Variables|LevelProperties|GetLevelDimensionsX)) (- (Variables|LevelProperties|GetLevelDimensionsX) 1))
                    (if (.Right (Utilities|Struct|BreakSTRUCT_ConnectedRooms (Utilities|Array|Get(acopy) (Variables|Default|GetConnectedRooms) (Variables|Default|GetCurrentRoom))))
                      (goto _label_9)
                      (else
                        (Utilities|Array|Add _movedirections_5 (Utilities|Array|Get(acopy) _roomplaced_2 (+ (Variables|Default|GetCurrentRoom) 1)))))
                    (else
                      (goto _label_9))))
                (:then_2
                  (if (>= (Variables|Default|GetCurrentRoom) (Variables|LevelProperties|GetLevelDimensionsX))
                    (if (.Up (Utilities|Struct|BreakSTRUCT_ConnectedRooms (Utilities|Array|Get(acopy) (Variables|Default|GetConnectedRooms) (Variables|Default|GetCurrentRoom))))
                      (goto _label_9)
                      (else
                        (Utilities|Array|Add _movedirections_5 (Utilities|Array|Get(acopy) _roomplaced_2 (- (Variables|Default|GetCurrentRoom) (Variables|LevelProperties|GetLevelDimensionsX))))))
                    (else
                      (goto _label_9))))
                (:then_3
                  (if (< (- (Variables|LevelProperties|GetLevelDimensionsY) 1) (* (Variables|LevelProperties|GetLevelDimensionsX) (- (Variables|LevelProperties|GetLevelDimensionsY) 1)))
                    (if (.Down (Utilities|Struct|BreakSTRUCT_ConnectedRooms (Utilities|Array|Get(acopy) (Variables|Default|GetConnectedRooms) (Variables|Default|GetCurrentRoom))))
                      (goto _label_9)
                      (else
                        (Utilities|Array|Add _movedirections_5 (Utilities|Array|Get(acopy) _roomplaced_2 (+ (Variables|Default|GetCurrentRoom) (Variables|LevelProperties|GetLevelDimensionsX))))))
                    (else
                      (goto _label_9))))
                (:then_4
                  (Utilities|CheckMoveOptions
                    (:Choose
                      (Variables|Movement|SetMovementChoice (Math|Random|RandomIntegerinRange 1 (Variables|Movement|GetNoOfMoveOptions)))
                      (for (_array_element_4 _array_index_2) (Variables|Movement|GetMoveDirections)
                        (if _array_element_4
                          (Variables|Default|SetMainLoopIndex _array_index_2)
                          (Variables|Movement|SetMovementDirectionSearch (+ (Variables|Movement|GetMovementDirectionSearch) 1))
                          (if (== (Variables|Movement|GetMovementDirectionSearch) (Variables|Movement|GetMovementChoice))
                            (Variables|Default|SetPreviousRoom (Utilities|Select :Index (Variables|Default|GetMainLoopIndex) :Option%200 (- (Variables|Default|GetCurrentRoom) 1) :Option%201 (+ (Variables|Default|GetCurrentRoom) 1) :Option%202 (- (Variables|Default|GetCurrentRoom) (Variables|LevelProperties|GetLevelDimensionsX)) :Option%203 (+ (Variables|Default|GetCurrentRoom) (Variables|LevelProperties|GetLevelDimensionsX))))
                            (Utilities|Array|SetArrayElem (Variables|Default|GetConnectedRooms) (Variables|Default|GetCurrentRoom) (Utilities|Select :Index (Variables|Default|GetMainLoopIndex) :Option%200 (Utilities|Struct|MakeSTRUCT_ConnectedRooms true (.Right (Utilities|Struct|BreakSTRUCT_ConnectedRooms (Utilities|Array|Get(acopy) (Variables|Default|GetConnectedRooms) (Variables|Default|GetCurrentRoom)))) (.Up (Utilities|Struct|BreakSTRUCT_ConnectedRooms (Utilities|Array|Get(acopy) (Variables|Default|GetConnectedRooms) (Variables|Default|GetCurrentRoom)))) (.Down (Utilities|Struct|BreakSTRUCT_ConnectedRooms (Utilities|Array|Get(acopy) (Variables|Default|GetConnectedRooms) (Variables|Default|GetCurrentRoom))))) :Option%201 (Utilities|Struct|MakeSTRUCT_ConnectedRooms (.Left (Utilities|Struct|BreakSTRUCT_ConnectedRooms (Utilities|Array|Get(acopy) (Variables|Default|GetConnectedRooms) (Variables|Default|GetCurrentRoom)))) true (.Up (Utilities|Struct|BreakSTRUCT_ConnectedRooms (Utilities|Array|Get(acopy) (Variables|Default|GetConnectedRooms) (Variables|Default|GetCurrentRoom)))) (.Down (Utilities|Struct|BreakSTRUCT_ConnectedRooms (Utilities|Array|Get(acopy) (Variables|Default|GetConnectedRooms) (Variables|Default|GetCurrentRoom))))) :Option%202 (Utilities|Struct|MakeSTRUCT_ConnectedRooms (.Left (Utilities|Struct|BreakSTRUCT_ConnectedRooms (Utilities|Array|Get(acopy) (Variables|Default|GetConnectedRooms) (Variables|Default|GetCurrentRoom)))) (.Right (Utilities|Struct|BreakSTRUCT_ConnectedRooms (Utilities|Array|Get(acopy) (Variables|Default|GetConnectedRooms) (Variables|Default|GetCurrentRoom)))) true (.Down (Utilities|Struct|BreakSTRUCT_ConnectedRooms (Utilities|Array|Get(acopy) (Variables|Default|GetConnectedRooms) (Variables|Default|GetCurrentRoom))))) :Option%203 (Utilities|Struct|MakeSTRUCT_ConnectedRooms (.Left (Utilities|Struct|BreakSTRUCT_ConnectedRooms (Utilities|Array|Get(acopy) (Variables|Default|GetConnectedRooms) (Variables|Default|GetCurrentRoom)))) (.Right (Utilities|Struct|BreakSTRUCT_ConnectedRooms (Utilities|Array|Get(acopy) (Variables|Default|GetConnectedRooms) (Variables|Default|GetCurrentRoom)))) (.Up (Utilities|Struct|BreakSTRUCT_ConnectedRooms (Utilities|Array|Get(acopy) (Variables|Default|GetConnectedRooms) (Variables|Default|GetCurrentRoom)))) true)))
                            (Utilities|Array|SetArrayElem (Variables|Default|GetConnectedRooms) (Variables|Default|GetPreviousRoom) (Utilities|Select :Index (Variables|Default|GetMainLoopIndex) :Option%200 (Utilities|Struct|MakeSTRUCT_ConnectedRooms (.Left (Utilities|Struct|BreakSTRUCT_ConnectedRooms (Utilities|Array|Get(acopy) (Variables|Default|GetConnectedRooms) (Variables|Default|GetPreviousRoom)))) true (.Up (Utilities|Struct|BreakSTRUCT_ConnectedRooms (Utilities|Array|Get(acopy) (Variables|Default|GetConnectedRooms) (Variables|Default|GetPreviousRoom)))) (.Down (Utilities|Struct|BreakSTRUCT_ConnectedRooms (Utilities|Array|Get(acopy) (Variables|Default|GetConnectedRooms) (Variables|Default|GetPreviousRoom))))) :Option%201 (Utilities|Struct|MakeSTRUCT_ConnectedRooms true (.Right (Utilities|Struct|BreakSTRUCT_ConnectedRooms (Utilities|Array|Get(acopy) (Variables|Default|GetConnectedRooms) (Variables|Default|GetPreviousRoom)))) (.Up (Utilities|Struct|BreakSTRUCT_ConnectedRooms (Utilities|Array|Get(acopy) (Variables|Default|GetConnectedRooms) (Variables|Default|GetPreviousRoom)))) (.Down (Utilities|Struct|BreakSTRUCT_ConnectedRooms (Utilities|Array|Get(acopy) (Variables|Default|GetConnectedRooms) (Variables|Default|GetPreviousRoom))))) :Option%202 (Utilities|Struct|MakeSTRUCT_ConnectedRooms (.Left (Utilities|Struct|BreakSTRUCT_ConnectedRooms (Utilities|Array|Get(acopy) (Variables|Default|GetConnectedRooms) (Variables|Default|GetPreviousRoom)))) (.Right (Utilities|Struct|BreakSTRUCT_ConnectedRooms (Utilities|Array|Get(acopy) (Variables|Default|GetConnectedRooms) (Variables|Default|GetPreviousRoom)))) (.Up (Utilities|Struct|BreakSTRUCT_ConnectedRooms (Utilities|Array|Get(acopy) (Variables|Default|GetConnectedRooms) (Variables|Default|GetPreviousRoom)))) true) :Option%203 (Utilities|Struct|MakeSTRUCT_ConnectedRooms (.Left (Utilities|Struct|BreakSTRUCT_ConnectedRooms (Utilities|Array|Get(acopy) (Variables|Default|GetConnectedRooms) (Variables|Default|GetPreviousRoom)))) (.Right (Utilities|Struct|BreakSTRUCT_ConnectedRooms (Utilities|Array|Get(acopy) (Variables|Default|GetConnectedRooms) (Variables|Default|GetPreviousRoom)))) true (.Down (Utilities|Struct|BreakSTRUCT_ConnectedRooms (Utilities|Array|Get(acopy) (Variables|Default|GetConnectedRooms) (Variables|Default|GetPreviousRoom)))))))
                            (Utilities|Array|Clear (Variables|Movement|GetMoveDirections))
                            (Variables|Movement|SetNoOfMoveOptions 0)
                            (Variables|Movement|SetMovementDirectionSearch 0)))))
                    (:Try%20Again
                      (if (< (Variables|Default|GetExtraConnectionAttempts) 32)
                        (Utilities|Array|Clear (Variables|Movement|GetMoveDirections))
                        (Variables|Movement|SetNoOfMoveOptions 0)
                        (goto _label_8)
                        (else
                          (Development|PrintString "ERROR: Can't Add Further Connections to Rooms")
                          (Utilities|Array|Clear (Variables|Movement|GetMoveDirections))
                          (Variables|Movement|SetNoOfMoveOptions 0)
                          (goto _label_7 Break))))))))))
        (:then_2
          (for _array_element_5 (Variables|Movement|GetStepsTaken)
            (Variables|Default|SetMainLoopIndex _array_element_5)
            (bind (_xcoord _ycoord) (CallFunction|1DArrayto2DCoords (Math|Conversions|ToFloat(Integer) (Variables|Default|GetMainLoopIndex)) (Math|Conversions|ToFloat(Integer) (Variables|LevelProperties|GetLevelDimensionsX))))
            (Variables|Default|SetCurrentRoomPos (Math|Vector|MakeVector (* _xcoord (.X (Math|Vector2D|BreakVector2D (Variables|LevelProperties|GetRoomDimensions)))) (* _ycoord (.Y (Math|Vector2D|BreakVector2D (Variables|LevelProperties|GetRoomDimensions)))) 0.0))
            (switch int (+ (Math|Conversions|ToInteger(Boolean) (.Left (Utilities|Struct|BreakSTRUCT_ConnectedRooms (Utilities|Array|Get(acopy) (Variables|Default|GetConnectedRooms) (Variables|Default|GetMainLoopIndex))))) (Math|Conversions|ToInteger(Boolean) (.Right (Utilities|Struct|BreakSTRUCT_ConnectedRooms (Utilities|Array|Get(acopy) (Variables|Default|GetConnectedRooms) (Variables|Default|GetMainLoopIndex))))) (Math|Conversions|ToInteger(Boolean) (.Up (Utilities|Struct|BreakSTRUCT_ConnectedRooms (Utilities|Array|Get(acopy) (Variables|Default|GetConnectedRooms) (Variables|Default|GetMainLoopIndex))))) (Math|Conversions|ToInteger(Boolean) (.Down (Utilities|Struct|BreakSTRUCT_ConnectedRooms (Utilities|Array|Get(acopy) (Variables|Default|GetConnectedRooms) (Variables|Default|GetMainLoopIndex))))))
              (:1
                ;[1 1 1] 1 Connected Room
                (if (.Left (Utilities|Struct|BreakSTRUCT_ConnectedRooms (Utilities|Array|Get(acopy) (Variables|Default|GetConnectedRooms) (Variables|Default|GetMainLoopIndex))))
                  (Variables|Default|SetRoomRotation 9e+01 :!label _label_10)
                  (elif (.Right (Utilities|Struct|BreakSTRUCT_ConnectedRooms (Utilities|Array|Get(acopy) (Variables|Default|GetConnectedRooms) (Variables|Default|GetMainLoopIndex))))
                    (Variables|Default|SetRoomRotation 2.7e+02)
                    (elif (.Up (Utilities|Struct|BreakSTRUCT_ConnectedRooms (Utilities|Array|Get(acopy) (Variables|Default|GetConnectedRooms) (Variables|Default|GetMainLoopIndex))))
                      (Variables|Default|SetRoomRotation 1.8e+02)
                      (elif (.Down (Utilities|Struct|BreakSTRUCT_ConnectedRooms (Utilities|Array|Get(acopy) (Variables|Default|GetConnectedRooms) (Variables|Default|GetMainLoopIndex))))
                        (Variables|Default|SetRoomRotation 0.0)
                        (else
                          (goto _label_10))))))
                (bind _returnvalue_2 (Game|SpawnActorfromClass "/Game/BP_LevelRoom_1Entry.BP_LevelRoom_1Entry_C" (Math|Transform|MakeTransform (+ (Variables|Default|GetCurrentRoomPos) (Variables|LevelProperties|GetStartingPos)) (Math|Rotator|MakeRotator 0.0 0.0 (Variables|Default|GetRoomRotation))) "Undefined" 0 0))
                (Utilities|Array|SetArrayElem (Variables|Default|GetRooms) (Variables|Default|GetMainLoopIndex) _returnvalue_2))
              (:2
                ;[1 1 1] 2 Connected Rooms
                (if (or (and (.Left (Utilities|Struct|BreakSTRUCT_ConnectedRooms (Utilities|Array|Get(acopy) (Variables|Default|GetConnectedRooms) (Variables|Default|GetMainLoopIndex)))) (.Right (Utilities|Struct|BreakSTRUCT_ConnectedRooms (Utilities|Array|Get(acopy) (Variables|Default|GetConnectedRooms) (Variables|Default|GetMainLoopIndex))))) (and (.Up (Utilities|Struct|BreakSTRUCT_ConnectedRooms (Utilities|Array|Get(acopy) (Variables|Default|GetConnectedRooms) (Variables|Default|GetMainLoopIndex)))) (.Down (Utilities|Struct|BreakSTRUCT_ConnectedRooms (Utilities|Array|Get(acopy) (Variables|Default|GetConnectedRooms) (Variables|Default|GetMainLoopIndex)))))) ; Corridor or Corner
                  (if (and (.Left (Utilities|Struct|BreakSTRUCT_ConnectedRooms (Utilities|Array|Get(acopy) (Variables|Default|GetConnectedRooms) (Variables|Default|GetMainLoopIndex)))) (.Right (Utilities|Struct|BreakSTRUCT_ConnectedRooms (Utilities|Array|Get(acopy) (Variables|Default|GetConnectedRooms) (Variables|Default|GetMainLoopIndex))))) ; Corridor: East-West or North-South
                    (Variables|Default|SetRoomRotation (Utilities|Select :Index _returnvalue :Option%200 9e+01 :Option%201 2.7e+02))
                    (else
                      (Variables|Default|SetRoomRotation (Utilities|Select :Index _returnvalue :Option%200 0.0 :Option%201 1.8e+02))))
                  (bind _returnvalue_3 (Game|SpawnActorfromClass "/Game/BP_LevelRoom_2EntryS.BP_LevelRoom_2EntryS_C" (Math|Transform|MakeTransform (+ (Variables|Default|GetCurrentRoomPos) (Variables|LevelProperties|GetStartingPos)) (Math|Rotator|MakeRotator 0.0 0.0 (Variables|Default|GetRoomRotation))) "Undefined" 0 0))
                  (Utilities|Array|SetArrayElem _rooms (Variables|Default|GetMainLoopIndex) _returnvalue_3)
                  (else
                    (if (and (.Left (Utilities|Struct|BreakSTRUCT_ConnectedRooms (Utilities|Array|Get(acopy) (Variables|Default|GetConnectedRooms) (Variables|Default|GetMainLoopIndex)))) (.Up (Utilities|Struct|BreakSTRUCT_ConnectedRooms (Utilities|Array|Get(acopy) (Variables|Default|GetConnectedRooms) (Variables|Default|GetMainLoopIndex)))))
                      (Variables|Default|SetRoomRotation 9e+01 :!label _label_11)
                      (elif (and (.Right (Utilities|Struct|BreakSTRUCT_ConnectedRooms (Utilities|Array|Get(acopy) (Variables|Default|GetConnectedRooms) (Variables|Default|GetMainLoopIndex)))) (.Up (Utilities|Struct|BreakSTRUCT_ConnectedRooms (Utilities|Array|Get(acopy) (Variables|Default|GetConnectedRooms) (Variables|Default|GetMainLoopIndex)))))
                        (Variables|Default|SetRoomRotation 1.8e+02)
                        (elif (and (.Right (Utilities|Struct|BreakSTRUCT_ConnectedRooms (Utilities|Array|Get(acopy) (Variables|Default|GetConnectedRooms) (Variables|Default|GetMainLoopIndex)))) (.Down (Utilities|Struct|BreakSTRUCT_ConnectedRooms (Utilities|Array|Get(acopy) (Variables|Default|GetConnectedRooms) (Variables|Default|GetMainLoopIndex)))))
                          (Variables|Default|SetRoomRotation 2.7e+02)
                          (elif (and (.Left (Utilities|Struct|BreakSTRUCT_ConnectedRooms (Utilities|Array|Get(acopy) (Variables|Default|GetConnectedRooms) (Variables|Default|GetMainLoopIndex)))) (.Down (Utilities|Struct|BreakSTRUCT_ConnectedRooms (Utilities|Array|Get(acopy) (Variables|Default|GetConnectedRooms) (Variables|Default|GetMainLoopIndex)))))
                            (Variables|Default|SetRoomRotation 0.0)
                            (else
                              (goto _label_11))))))
                    (bind _returnvalue_4 (Game|SpawnActorfromClass "/Game/BP_LevelRoom_2EntryC.BP_LevelRoom_2EntryC_C" (Math|Transform|MakeTransform (+ (Variables|Default|GetCurrentRoomPos) (Variables|LevelProperties|GetStartingPos)) (Math|Rotator|MakeRotator 0.0 0.0 (Variables|Default|GetRoomRotation))) "Undefined" 0 0))
                    (Utilities|Array|SetArrayElem _rooms (Variables|Default|GetMainLoopIndex) _returnvalue_4))))
              (:3
                ;[1 1 1] 3 Connected Rooms
                (if (.Left (Utilities|Struct|BreakSTRUCT_ConnectedRooms (Utilities|Array|Get(acopy) (Variables|Default|GetConnectedRooms) (Variables|Default|GetMainLoopIndex))))
                  (if (.Right (Utilities|Struct|BreakSTRUCT_ConnectedRooms (Utilities|Array|Get(acopy) (Variables|Default|GetConnectedRooms) (Variables|Default|GetMainLoopIndex))))
                    (if (.Up (Utilities|Struct|BreakSTRUCT_ConnectedRooms (Utilities|Array|Get(acopy) (Variables|Default|GetConnectedRooms) (Variables|Default|GetMainLoopIndex))))
                      (if (.Down (Utilities|Struct|BreakSTRUCT_ConnectedRooms (Utilities|Array|Get(acopy) (Variables|Default|GetConnectedRooms) (Variables|Default|GetMainLoopIndex))))
                        (Variables|Default|SetRoomRotation 1.8e+02 :!label _label_12)
                        (else
                          (Variables|Default|SetRoomRotation 9e+01)))
                      (else
                        (Variables|Default|SetRoomRotation 2.7e+02)))
                    (else
                      (Variables|Default|SetRoomRotation 0.0)))
                  (else
                    (goto _label_12)))
                (bind _returnvalue_5 (Game|SpawnActorfromClass "/Game/BP_LevelRoom_3Entry.BP_LevelRoom_3Entry_C" (Math|Transform|MakeTransform (+ (Variables|Default|GetCurrentRoomPos) (Variables|LevelProperties|GetStartingPos)) (Math|Rotator|MakeRotator 0.0 0.0 (Variables|Default|GetRoomRotation))) "Undefined" 0 0))
                (Utilities|Array|SetArrayElem (Variables|Default|GetRooms) (Variables|Default|GetMainLoopIndex) _returnvalue_5))
              (:4
                ;[1 1 1] 4 Connected Rooms
                (Variables|Default|SetRoomRotation 0.0)
                (bind _returnvalue_6 (Game|SpawnActorfromClass "/Game/BP_LevelRoom_4Entry.BP_LevelRoom_4Entry_C" (Math|Transform|MakeTransform (+ (Variables|Default|GetCurrentRoomPos) (Variables|LevelProperties|GetStartingPos)) (Math|Rotator|MakeRotator 0.0 0.0 (Variables|Default|GetRoomRotation))) "Undefined" 0 0))
                (Utilities|Array|SetArrayElem (Variables|Default|GetRooms) (Variables|Default|GetMainLoopIndex) _returnvalue_6)))))
        (:then_3
          (Development|ExecuteConsoleCommand "RebuildNavigation" 0))))))

(fn ConstructionScript)

(fn 2DCoordsto1DArray
  (params (XCoord :type Integer) (YCoord :type Integer) (XDimension :type Integer))
  (return (+ XCoord (* YCoord XDimension))))

(fn 1DArrayto2DCoords
  (params (1DArray :type Float%20%28single-precision%29) (XDimension :type Float%20%28single-precision%29))
  (bind _returnvalue (/ 1DArray XDimension))
  (bind _returnvalue_2 (Math|Float|Floor _returnvalue))
  (return (Math|Float|Floor (- 1DArray (* _returnvalue_2 XDimension))) _returnvalue_2))